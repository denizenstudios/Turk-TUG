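; Turk_Char_BP is a player character Blueprint that handles gamepad camera look and axis-driven movement.
; Turn and look axes add controller yaw and pitch, scaled by TurnRateGamePad and frame delta time for frame-rate independence.
; Both movement axes add input along a yaw-only vector from control rotation, with Move Right / Left also using the forward vector rather than a right vector.
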(event Input|AxisEvents|InputAxisTurnRight/LeftGamepad
  (params (AxisValue :type Float%20%28single-precision%29))
  ;[1 1 1] Camera Input - Game Pad
  (Pawn|Input|AddControllerYawInput (* AxisValue (Variables|Default|GetTurnRateGamePad) (Utilities|Time|GetWorldDeltaSeconds))))

(event Input|AxisEvents|InputAxisLookUp/DownGamepad
  (params (AxisValue :type Float%20%28single-precision%29))
  ;[1 1 1] Camera Input - Game Pad
  (Pawn|Input|AddControllerPitchInput (* AxisValue (Variables|Default|GetTurnRateGamePad) (Utilities|Time|GetWorldDeltaSeconds))))

(event Input|AxisEvents|InputAxisMoveForward/Backward
  (params (AxisValue :type Float%20%28single-precision%29))
  (Pawn|Input|AddMovementInput (Math|Vector|GetForwardVector (Math|Rotator|MakeRotator 0.0 0.0 (.yaw (Pawn|GetControlRotation :!class /Script/Engine.Pawn)))) AxisValue false))

(event Input|AxisEvents|InputAxisMoveRight/Left
  (params (AxisValue :type Float%20%28single-precision%29))
  (Pawn|Input|AddMovementInput (Math|Vector|GetForwardVector (Math|Rotator|MakeRotator 0.0 0.0 (.yaw (Pawn|GetControlRotation :!class /Script/Engine.Pawn)))) AxisValue false))

(fn ConstructionScript)