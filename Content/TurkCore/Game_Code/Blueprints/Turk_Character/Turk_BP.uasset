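; Turk player character Blueprint handling movement and interaction with nearby objects.
; Move axes add control-yaw-based input and call PlayerDir, which turns the actor toward a world-space input vector and adds movement along it.
; InteractRadius overlaps track one highlighted BP_Interactable, which E triggers before switching to UI-only input with a cursor.
; RotateToFaceCursor is defined but uncalled, and an NPC dialog overlap loop is disconnected.
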(event OnComponentBeginOverlap(interactRadius)
  (params (OverlappedComponent :type Primitive%20Component%20Object%20Reference) (OtherActor :type Actor%20Object%20Reference) (OtherComp :type Primitive%20Component%20Object%20Reference) (OtherBodyIndex :type Integer) (bFromSweep :type Boolean) (SweepResult :type Hit%20Result%20Structure%20%28by%20ref%29))
  (if (!= OtherActor self)
    (if (Utilities|DoesObjectImplementInterface OtherActor "/Game/TurkCore/Game_Code/Blueprints/NPCs/npc_interact/dialogue2/BP_Interactable.BP_Interactable_C")
      (Utilities|IsValid (Variables|Default|Getinteractable)
        (:Is%20Valid
          (Class|BPInteractable|SetInteractableState(Message) (Variables|Default|Getinteractable) false)
          (Variables|Default|Setinteractable 0))
        (:Is%20Not%20Valid
          _))
      (Variables|Default|Setinteractable OtherActor)
      (Class|BPInteractable|SetInteractableState(Message) (Variables|Default|Getinteractable) true))))

(event OnComponentEndOverlap(interactRadius)
  (params (OverlappedComponent :type Primitive%20Component%20Object%20Reference) (OtherActor :type Actor%20Object%20Reference) (OtherComp :type Primitive%20Component%20Object%20Reference) (OtherBodyIndex :type Integer))
  (if (and (!= 0 self) (== (Variables|Default|Getinteractable) OtherActor))
    (Class|BPInteractable|SetInteractableState(Message) (Variables|Default|Getinteractable) false)
    (Variables|Default|Setinteractable 0)))

(event Input|AxisEvents|InputAxisMoveForward/Backward
  (params (AxisValue :type Float%20%28single-precision%29))
  ;[1 1 1] Movement
  (CallFunction|PlayerDir)
  (Pawn|Input|AddMovementInput (Math|Vector|GetForwardVector (Math|Rotator|MakeRotator 0.0 0.0 (.yaw (Pawn|GetControlRotation :!class /Script/Engine.Pawn)))) AxisValue false))

(event Input|AxisEvents|InputAxisMoveRight/Left
  (params (AxisValue :type Float%20%28single-precision%29))
  (bind _returnvalue (Pawn|GetControlRotation :!class /Script/Engine.Pawn))
  ;[1 1 1] Movement
  (CallFunction|PlayerDir)
  (Pawn|Input|AddMovementInput (Math|Vector|GetRightVector (Math|Rotator|MakeRotator (.roll _returnvalue) 0.0 (.yaw _returnvalue))) AxisValue false))

(event Input|KeyboardEvents|E
  (params (Key :type Key%20Structure :default "None"))
  (:Pressed
    (Utilities|IsValid (Variables|Default|Getinteractable)
      (:Is%20Valid
        (Class|BPInteractable|Interact(Message) (Variables|Default|Getinteractable) self)
        (Input|SetInputModeUIOnly (Game|GetPlayerController 0) 0 "DoNotLock")
        (Variables|/Script/Engine.PlayerController|SetbShowMouseCursor (Game|GetPlayerController 0) true)))))

(fn ConstructionScript)

(fn RotatetoFaceCursor
  (bind _returnvalue (Game|GetPlayerController 0))
  (Pawn|SetControlRotation _returnvalue (Math|Rotator|MakeRotator 0.0 0.0 (.yaw (Math|Rotator|FindLookatRotation (Transformation|GetActorLocation self) (.Location (Collision|BreakHitResult (.HitResult (Game|Player|GetHitResultUnderCursorbyChannel _returnvalue "TraceTypeQuery1" true)))))))))

(fn PlayerDir
  (bind _output_get (Variables|Default|SetMove%20Direction (Math|Vector|Normalize (Math|Vector|MakeVector (Input|AxisValues|GetMoveForward/Backward) (Input|AxisValues|GetMoveRight/Left) 0.0))))
  (if (> (Math|Vector|VectorLength _output_get) 0.05)
    (Transformation|SetActorRotation self (Math|Rotator|MakeRotfromX (Variables|Default|GetMove%20Direction)))
    (Pawn|Input|AddMovementInput (Variables|Default|GetMove%20Direction) 1.0 false)
    (Variables|Default|SetbUseControllerRotationYaw false)))