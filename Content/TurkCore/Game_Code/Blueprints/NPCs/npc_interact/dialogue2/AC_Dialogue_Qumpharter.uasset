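; Dialogue component for the NPC Qumpharter, who asks the player to clear an infestation from his spaceship.
; It extends a parent Dialogue function and branches on the dialogue tree index and the chosen option.
; Accepting closes the conversation, opens the SpaceShooter level and restores game-only input.
; Declining shows a short reply, then clears dialogue progress, closes the conversation and restores game-only input.
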(fn Dialogue
  (|CallParentFunction)
  (switch int (Variables|Default|GetdialogueTreeIndex)
    (:0
      (bind (_state _optionindex) (CallFunction|AddDialogue "Qumpharter" "Can you please clear the infestation from my spaceship?" (Utilities|Array|MakeArray "Yes I can! No prob" "Uhhhh nah Im cool")))
      (switch Utilities|FlowControl|Switch|SwitchonEnum_Dialogue_State _state
        (:NewEnumerator0
          (switch int _optionindex
            (:0
              (CallFunction|CloseConversation)
              (Game|OpenLevel(byObjectReference) "/Game/TurkCore/Maps/spaceShooter.spaceShooter")
              (Input|SetInputModeGameOnly (Game|GetPlayerController 0)))
            (:1
              (bind _state_2 (CallFunction|AddDialogue "Qumpharter" "Oh okay :(" (Utilities|Array|MakeArray "bye!")))
              (switch Utilities|FlowControl|Switch|SwitchonEnum_Dialogue_State _state_2
                (:NewEnumerator0
                  (CallFunction|ClearDialogueProgress)
                  (CallFunction|CloseConversation)
                  (Input|SetInputModeGameOnly (Game|GetPlayerController 0)))))))))))