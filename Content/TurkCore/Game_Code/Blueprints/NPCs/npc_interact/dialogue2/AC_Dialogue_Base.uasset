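; Base dialogue component for NPC conversations that opens and closes a W_Dialogue widget and tracks the player's choices.
; The empty Dialogue function, presumably overridden per conversation, is re-run from the start on every progression.
; AddDialogue returns stored choices for answered steps and displays the first unanswered one in the widget.
; UpdateSelectedOption records choices and triggers the replay; helpers clear or rewind progress, or switch dialogue trees.
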(fn OpenConversation
  (bind _returnvalue (UserInterface|CreateWidget "/Game/TurkCore/Game_Code/Interface/W_Dialogue.W_Dialogue_C" 0 self))
  (bind _output_get (Variables|Default|SetdialogueWidget _returnvalue))
  (UserInterface|Viewport|AddtoViewport _output_get 0)
  (CallFunction|ProgressDialogue))

(fn CloseConversation
  (Widget|RemovefromParent (Variables|Default|GetdialogueWidget)))

(fn ProgressDialogue
  (Variables|Default|SetdialogueIndex -1)
  (CallFunction|Dialogue))

(fn Dialogue)

(fn AddDialogue
  (params (speaker :type Text) (dialogue :type Text) (optionsText :type Array%20of%20Texts))
  (bind _dialogueprogress (Variables|Default|GetdialogueProgress))
  (bind _dialogueindex (Variables|Default|GetdialogueIndex))
  (bind (_value _returnvalue) (Utilities|Map|Find _dialogueprogress _dialogueindex))
  (Math|Integer|IncrementInt (Variables|Default|GetdialogueIndex)
    (:%20%20
      (if _returnvalue
        (return "NewEnumerator0" _value)
        (else
          (Default|UpdateDialogueText (Variables|Default|GetdialogueWidget) (Variables|Default|GetdialogueIndex) speaker dialogue optionsText)
          (return "NewEnumerator1" 0))))))

(fn UpdateSelectedOption
  (params (progessIndex :type Integer%20%28by%20ref%29) (optionIndex :type Integer%20%28by%20ref%29))
  (Utilities|Map|Add (Variables|Default|GetdialogueProgress) progessIndex optionIndex)
  (CallFunction|ProgressDialogue))

(fn ClearDialogueProgress
  (Utilities|Map|Clear (Variables|Default|GetdialogueProgress)))

(fn RemoveDialogueProgress
  (params (progressSteps :type Integer))
  (for _index (range 0 progressSteps)
    (Utilities|Map|Remove (Variables|Default|GetdialogueProgress) (- (Variables|Default|GetdialogueIndex) _index))))

(fn SetDialogueTreeIndex
  (params (dialogueTreeIndex :type Integer))
  (Variables|Default|SetdialogueTreeIndex dialogueTreeIndex)
  (CallFunction|ClearDialogueProgress))